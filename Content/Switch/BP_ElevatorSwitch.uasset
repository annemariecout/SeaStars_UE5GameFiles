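; BP_ElevatorSwitch is an elevator the player rides between a start and end point by using a switch while standing in its trigger box.
; Overlapping the box flags the player as aboard and binds the elevator's use event to the character through AssignUseSwitch.
; Using it plays or reverses a timeline that lerps the elevator's relative location, choosing direction by whether it sits exactly at the end point.
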(event OnComponentBeginOverlap(BoxTrigger)
  (params (OverlappedComponent :type Primitive%20Component%20Object%20Reference) (OtherActor :type Actor%20Object%20Reference) (OtherComp :type Primitive%20Component%20Object%20Reference) (OtherBodyIndex :type Integer) (bFromSweep :type Boolean) (SweepResult :type Hit%20Result%20Structure%20%28by%20ref%29))
  (if (== OtherActor (Variables|Default|GetTP%20Char%20Ref))
    (Variables|Default|SetOnElevator true)
    (CallFunction|RideUp)))

(event OnComponentEndOverlap(BoxTrigger)
  (params (OverlappedComponent :type Primitive%20Component%20Object%20Reference) (OtherActor :type Actor%20Object%20Reference) (OtherComp :type Primitive%20Component%20Object%20Reference) (OtherBodyIndex :type Integer))
  (if (== OtherActor (Variables|Default|GetTP%20Char%20Ref))
    (Variables|Default|SetOnElevator false)))

(event Custom|ElevatorUse
  (if (Variables|Default|GetOnElevator)
    (if (Utilities|Operators|EqualEqual (Variables|/Script/Engine.SceneComponent|GetRelativeLocation (Variables|Default|GetElevator)) (Variables|Default|GetEndPoint) 0.0)
      (bind _movementfloat (Timeline|ElevatorMove Reverse)
        (:Update
          (Transformation|SetRelativeLocation (Variables|Default|GetElevator) (Math|Vector|Lerp(Vector) (Variables|Default|GetStartPoint) (Variables|Default|GetEndPoint) _movementfloat) false false)))
      (else
        (Timeline|ElevatorMove Play)))))

(event Custom|RideUp
  (EventDispatchers|AssignUseSwitch (Variables|Default|GetTP%20Char%20Ref) (delegate Custom|ElevatorUse)))

(event EventBeginPlay
  (bind _asbp_third_person_character (Utilities|Casting|CastToBP_ThirdPersonCharacter (Game|Player|GetPlayerPawn 0)))
  (Variables|Default|SetTP%20Char%20Ref _asbp_third_person_character))

(fn ConstructionScript)