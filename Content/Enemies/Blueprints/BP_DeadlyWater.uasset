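; BP_DeadlyWater is a hazard volume that repeatedly damages the player character while it is inside the water.
; BeginPlay caches the player as BP_ThirdPersonCharacter, and box overlap events for that character toggle IsInWater and call InWater.
; InWater loops through a short Delay, applying damage while the flag holds, and calls TPCharDead when HealthAmt equals exactly zero after a delay.
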(event OnComponentBeginOverlap(BoxCollision)
  (params (OverlappedComponent :type Primitive%20Component%20Object%20Reference) (OtherActor :type Actor%20Object%20Reference) (OtherComp :type Primitive%20Component%20Object%20Reference) (OtherBodyIndex :type Integer) (bFromSweep :type Boolean) (SweepResult :type Hit%20Result%20Structure%20%28by%20ref%29))
  (if (== OtherActor (Variables|Default|GetTP%20Char%20Ref))
    (Variables|Default|SetIsInWater? true)
    (CallFunction|InWater)))

(event OnComponentEndOverlap(BoxCollision)
  (params (OverlappedComponent :type Primitive%20Component%20Object%20Reference) (OtherActor :type Actor%20Object%20Reference) (OtherComp :type Primitive%20Component%20Object%20Reference) (OtherBodyIndex :type Integer))
  (if (== OtherActor (Variables|Default|GetTP%20Char%20Ref))
    (Variables|Default|SetIsInWater? false)
    (CallFunction|InWater)))

(event Custom|InWater
  (if (Variables|Default|GetIsInWater?) :!label _label
    (Game|Damage|ApplyDamage (Variables|Default|GetTP%20Char%20Ref) 1e+01 0 self)
    (Utilities|FlowControl|Delay 0.3)
    (if (== (Variables|/Game/ThirdPerson/Blueprints/BP_ThirdPersonCharacter.BP_ThirdPersonCharacter_C|GetHealthAmt (Variables|Default|GetTP%20Char%20Ref)) 0.0)
      (Default|TPCharDead (Variables|Default|GetTP%20Char%20Ref))
      (else
        (goto _label)))))

(event EventBeginPlay
  (bind _asbp_third_person_character (Utilities|Casting|CastToBP_ThirdPersonCharacter (Game|Player|GetPlayerPawn 0)))
  (Variables|Default|SetTP%20Char%20Ref _asbp_third_person_character))

(fn ConstructionScript)