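; BP_Elevator is an elevator that rises once its bosses are gone and carries the player while they stand on it.
; At BeginPlay it registers itself with each BossRef entry; CheckAndMoveElevator eases it to a fixed height with a bubble sound when that array is empty.
; Box trigger overlaps by the player play or reverse, after a short delay, a timeline lerping the platform between StartPoint and EndPoint.
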(event OnComponentBeginOverlap(BoxTrigger)
  (params (OverlappedComponent :type Primitive%20Component%20Object%20Reference) (OtherActor :type Actor%20Object%20Reference) (OtherComp :type Primitive%20Component%20Object%20Reference) (OtherBodyIndex :type Integer) (bFromSweep :type Boolean) (SweepResult :type Hit%20Result%20Structure%20%28by%20ref%29))
  (if (== OtherActor (Variables|Default|GetTP%20Char%20Ref))
    (Variables|Default|SetOnElevator true)
    (Utilities|FlowControl|Delay 0.5)
    (CallFunction|ElevatorUse)))

(event OnComponentEndOverlap(BoxTrigger)
  (params (OverlappedComponent :type Primitive%20Component%20Object%20Reference) (OtherActor :type Actor%20Object%20Reference) (OtherComp :type Primitive%20Component%20Object%20Reference) (OtherBodyIndex :type Integer))
  (if (== OtherActor (Variables|Default|GetTP%20Char%20Ref))
    (Variables|Default|SetOnElevator false)
    (Utilities|FlowControl|Delay 0.5)
    (CallFunction|ElevatorUse)))

(event Custom|CheckAndMoveElevator
  (if (== (Utilities|Array|Length (Variables|Default|GetBoss%20Ref)) 0)
    (CallFunction|MoveElevatorAnim)))

(event Custom|MoveElevatorAnim
  (bind _elevator (Variables|Default|GetElevator))
  (bind _relativelocation (Variables|/Script/Engine.SceneComponent|GetRelativeLocation _elevator))
  (Audio|PlaySoundatLocation "/Game/Sounds/Bubbles.Bubbles" "0, 0, 0" "0, 0, 0" 1.0 1.0 0.0 0 0 0 0)
  (Components|MoveComponentTo _elevator (Math|Vector|MakeVector (.x _relativelocation) (.y _relativelocation) 2.5e+02) (Variables|/Script/Engine.SceneComponent|GetRelativeRotation _elevator) true true 6.0 false))

(event Custom|ElevatorUse
  (if (Variables|Default|GetOnElevator)
    (bind _movementfloat (Timeline|ElevatorMove Play)
      (:Update
        (Transformation|SetRelativeLocation (Variables|Default|GetElevator) (Math|Vector|Lerp(Vector) (Variables|Default|GetStartPoint) (Variables|Default|GetEndPoint) _movementfloat) false false)))
    (else
      (Timeline|ElevatorMove Reverse))))

(event EventBeginPlay
  (Utilities|FlowControl|Sequence
    (:then_0
      (bind _asbp_third_person_character (Utilities|Casting|CastToBP_ThirdPersonCharacter (Game|Player|GetPlayerPawn 0)))
      (Variables|Default|SetTP%20Char%20Ref _asbp_third_person_character))
    (:then_1
      (for _array_element (Variables|Default|GetBoss%20Ref)
        (Variables|/Game/Enemies/Blueprints/BP_EnemyBoss.BP_EnemyBoss_C|SetElevator%20Ref _array_element self)))))

(fn ConstructionScript)