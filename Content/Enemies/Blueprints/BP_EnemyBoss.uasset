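; Boss enemy that wakes when pawn sensing spots the player, then chases and keeps turning to face them via delay loops.
; It deals contact damage on capsule hits with a one-second cooldown, and only takes damage once awake.
; Death triggers the referenced elevator and destroys the actor.
; A timer shows and aims its health widget at the player camera during the fight, while a replayed timeline bobs the Smoke component.
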(event OnSeePawn(PawnSensing)
  (params (Pawn :type Pawn%20Object%20Reference))
  ;[1 1 1] See Player?
  (bind _asbp_third_person_character (Utilities|Casting|CastToBP_ThirdPersonCharacter Pawn))
  (Utilities|FlowControl|Sequence
    (:then_0
      (Utilities|FlowControl|DoOnce false
        (:Completed
          (Variables|Default|SetIsReadyToFight true))))
    (:then_1
      (bind _output_get (Variables|Default|SetTP%20Char%20Ref _asbp_third_person_character))
      (if (not (or (Variables|/Game/ThirdPerson/Blueprints/BP_ThirdPersonCharacter.BP_ThirdPersonCharacter_C|GetIsDead? _output_get) (Variables|Default|GetIsEnemyDead?))) :!label _label
        (CallFunction|BossLookat)
        (AI|AIMoveTo self "0, 0, 0" (Variables|Default|GetTP%20Char%20Ref) 1e+02 false
          (:then
            (Utilities|FlowControl|Delay 0.1)
            (goto _label)))))))

(event OnComponentHit(CapsuleComponent)
  (params (HitComponent :type Primitive%20Component%20Object%20Reference) (OtherActor :type Actor%20Object%20Reference) (OtherComp :type Primitive%20Component%20Object%20Reference) (NormalImpulse :type Vector :default "0, 0, 0") (Hit :type Hit%20Result%20Structure%20%28by%20ref%29))
  ;[1 1 1] Damage when Character Overlaps
  (bind _asbp_third_person_character (Utilities|Casting|CastToBP_ThirdPersonCharacter OtherActor))
  (Utilities|FlowControl|DoOnce false :!label _label
    (:Completed
      (Default|TPCharRecieveDamage _asbp_third_person_character 2e+01 (Transformation|GetActorLocation))
      (Utilities|FlowControl|Delay 1.0)
      (goto _label Reset))))

(event Custom|BossReceiveDamage
  (params (Damage :type Float%20%28double-precision%29) (AttackType :type Float%20%28double-precision%29))
  ;[1 1 1] Damage System
  (if (Variables|Default|GetIsReadyToFight)
    (if (not (Variables|Default|GetIsEnemyDead?))
      (Variables|Default|SetCurrentHealth (- (Variables|Default|GetCurrentHealth) Damage))
      (if (<= (Variables|Default|GetCurrentHealth) 0.0)
        (CallFunction|BossDead)))))

(event Custom|BossDead
  (bind _elevator_ref (Variables|Default|GetElevator%20Ref))
  ;[1 1 1] Damage System
  (Utilities|IsValid _elevator_ref
    (:Is%20Valid
      (Default|CheckandMoveElevator _elevator_ref))
    (:Is%20Not%20Valid
      _))
  (Variables|Default|SetIsEnemyDead? true)
  (Variables|Default|SetIsReadyToFight false)
  (Variables|/Script/AIModule.PawnSensingComponent|SetbSeePawns (Variables|Default|GetPawnSensing) false)
  (Components|Movement|StopMovementImmediately (Variables|Character|GetCharacterMovement))
  (Actor|DestroyActor))

(event Custom|BossLookAt
  ;[1 1 1] Look At Player
  (Utilities|FlowControl|DoOnce false
    (:Completed
      (if (not (Variables|Default|GetIsEnemyDead?)) :!label _label
        (Transformation|SetActorRotation (Math|Rotator|MakeRotator 0.0 0.0 (.yaw (Math|Interpolation|RInterpTo (Transformation|GetActorRotation) (Math|Rotator|FindLookatRotation (Transformation|GetActorLocation) (Transformation|GetActorLocation (Game|GetPlayerCharacter 0))) (Utilities|Time|GetWorldDeltaSeconds) 3.0))))
        (Utilities|FlowControl|Delay 0.01)
        (goto _label)))))

(event Custom|StartTransform)

(event Custom|BossFloating
  (bind _smoke (Variables|Default|GetSmoke))
  (bind _relativelocation (Variables|/Script/Engine.SceneComponent|GetRelativeLocation _smoke))
  (bind _float (Timeline|FloatTimeline PlayFromStart)
    (:Update
      (Transformation|SetRelativeLocation _smoke (Math|Vector|MakeVector (.x _relativelocation) (.y _relativelocation) _float) false false))
    (:Finished
      (Utilities|FlowControl|Delay 0.01)
      (CallFunction|BossFloating))))

(event Custom|CheckBHealthWidget
  (bind _bosshealthwidget (Variables|Default|GetBossHealthWidget))
  (bind _bosshealthwidget_2 (Variables|Default|GetBossHealthWidget))
  ;[1 1 1] WBP
  (if (Variables|Default|GetIsReadyToFight)
    (if (Variables|Default|GetIsEnemyDead?)
      (Development|SetHiddeninGame _bosshealthwidget true false)
      (else
        (Development|SetHiddeninGame _bosshealthwidget false false)
        (bind _asbp_third_person_character (Utilities|Casting|CastToBP_ThirdPersonCharacter (Game|GetPlayerCharacter 0)))
        (Transformation|SetWorldRotation _bosshealthwidget_2 (Math|Rotator|MakeRotator 0.0 0.0 (.yaw (Math|Rotator|FindLookatRotation (Transformation|GetWorldLocation _bosshealthwidget_2) (Transformation|GetWorldLocation (Variables|/Game/ThirdPerson/Blueprints/BP_ThirdPersonCharacter.BP_ThirdPersonCharacter_C|GetFollowCamera _asbp_third_person_character))))) false false)))
    (else
      (Development|SetHiddeninGame _bosshealthwidget true false))))

(event Custom|WBPBoss
  ;[1 1 1] WBP
  (bind _aswbp_enemy_boss (Utilities|Casting|CastToWBP_EnemyBoss (UserInterface|GetUserWidgetObject (Variables|Default|GetBossHealthWidget))))
  (Variables|/Game/Enemies/Blueprints/WBP_EnemyBoss.WBP_EnemyBoss_C|SetBoss%20Ref _aswbp_enemy_boss self)
  (Utilities|Time|SetTimerbyEvent (delegate Custom|CheckBHealthWidget) 0.02 true))

(event EventBeginPlay
  (CallFunction|BossFloating)
  (CallFunction|WBPBoss))

(fn ConstructionScript)