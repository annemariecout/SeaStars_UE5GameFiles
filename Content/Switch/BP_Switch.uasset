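; BP_Switch is a switch the third-person player character can use to toggle its button between on and off looks.
; Entering BoxTrigger sets the character's CanUseSwitch flag and binds the switch's UseSwitch event to the character's UseSwitch dispatcher.
; Each use flip-flops SwitchButton between dynamic instances of the on and off materials, boosting emissive when on.
; Leaving the trigger neither clears the flag nor unbinds the event.
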(event OnComponentBeginOverlap(BoxTrigger)
  (params (OverlappedComponent :type Primitive%20Component%20Object%20Reference) (OtherActor :type Actor%20Object%20Reference) (OtherComp :type Primitive%20Component%20Object%20Reference) (OtherBodyIndex :type Integer) (bFromSweep :type Boolean) (SweepResult :type Hit%20Result%20Structure%20%28by%20ref%29))
  (bind _tp_char_ref (Variables|Default|GetTP%20Char%20Ref))
  (if (== OtherActor _tp_char_ref)
    (Variables|/Game/ThirdPerson/Blueprints/BP_ThirdPersonCharacter.BP_ThirdPersonCharacter_C|SetCanUseSwitch _tp_char_ref true)
    (CallFunction|SwitchPressed)))

(event OnComponentEndOverlap(BoxTrigger)
  (params (OverlappedComponent :type Primitive%20Component%20Object%20Reference) (OtherActor :type Actor%20Object%20Reference) (OtherComp :type Primitive%20Component%20Object%20Reference) (OtherBodyIndex :type Integer))
  (if (== OtherActor (Variables|Default|GetTP%20Char%20Ref))
    _))

(event Custom|SwitchPressed
  (EventDispatchers|AssignUseSwitch (Variables|Default|GetTP%20Char%20Ref) (delegate Custom|UseSwitch)))

(event Custom|UseSwitch
  (bind _switchbutton (Variables|Default|GetSwitchButton))
  (Utilities|FlowControl|FlipFlop
    (:A
      (bind _returnvalue (Rendering|Material|CreateDynamicMaterialInstance _switchbutton 0 "/Game/Switch/MI_SwitchOn.MI_SwitchOn" "None" :!class /Script/Engine.PrimitiveComponent))
      (Rendering|Material|SetScalarParameterValue _returnvalue "Emissive Boost" 2e+01 :!class /Script/Engine.MaterialInstanceDynamic))
    (:B
      (Rendering|Material|CreateDynamicMaterialInstance _switchbutton 0 "/Game/Switch/MI_SwitchOff.MI_SwitchOff" "None" :!class /Script/Engine.PrimitiveComponent))))

(event EventBeginPlay
  (bind _asbp_third_person_character (Utilities|Casting|CastToBP_ThirdPersonCharacter (Game|Player|GetPlayerPawn 0)))
  (Variables|Default|SetTP%20Char%20Ref _asbp_third_person_character))

(fn ConstructionScript)