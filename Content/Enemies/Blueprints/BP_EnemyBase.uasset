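; Base enemy that chases the player on sight, deals contact damage and is destroyed when its health runs out.
; Pawn sensing arms it to take damage, then delay loops repeat AIMoveTo and smoothly yaw it toward the player; capsule hits damage on a cooldown.
; A looping timer shows the health widget during combat and faces it to the camera, while a timeline bobs the smoke.
; Montage attack, elevator and level-up logic are disconnected.
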(event OnSeePawn(PawnSensing)
  (params (Pawn :type Pawn%20Object%20Reference))
  ;[1 1 1] See Player?
  (bind _asbp_third_person_character (Utilities|Casting|CastToBP_ThirdPersonCharacter Pawn))
  (Utilities|FlowControl|Sequence
    (:then_0
      (Utilities|FlowControl|DoOnce false
        (:Completed
          (Variables|Default|SetIsReadyToFight true))))
    (:then_1
      (bind _output_get (Variables|Default|SetTP%20Char%20Ref _asbp_third_person_character))
      (if (not (or (Variables|/Game/ThirdPerson/Blueprints/BP_ThirdPersonCharacter.BP_ThirdPersonCharacter_C|GetIsDead? _output_get) (Variables|Default|GetIsEnemyDead?))) :!label _label
        (CallFunction|Lookat)
        (AI|AIMoveTo self "0, 0, 0" (Variables|Default|GetTP%20Char%20Ref) 1e+02 false
          (:then
            (Utilities|FlowControl|Delay 0.1)
            (goto _label)))))))

(event OnComponentHit(CapsuleComponent)
  (params (HitComponent :type Primitive%20Component%20Object%20Reference) (OtherActor :type Actor%20Object%20Reference) (OtherComp :type Primitive%20Component%20Object%20Reference) (NormalImpulse :type Vector :default "0, 0, 0") (Hit :type Hit%20Result%20Structure%20%28by%20ref%29))
  ;[1 1 1] Damage when Character Overlaps
  (bind _asbp_third_person_character (Utilities|Casting|CastToBP_ThirdPersonCharacter OtherActor))
  (Utilities|FlowControl|DoOnce false :!label _label
    (:Completed
      (Default|TPCharRecieveDamage _asbp_third_person_character 2e+01 (Transformation|GetActorLocation))
      (Utilities|FlowControl|Delay 1.0)
      (goto _label Reset))))

(event Custom|EnemyReceiveDamage
  (params (Damage :type Float%20%28double-precision%29) (AttackType :type Float%20%28double-precision%29))
  ;[1 1 1] Damage System
  (if (Variables|Default|GetIsReadyToFight)
    (if (not (Variables|Default|GetIsEnemyDead?))
      (Variables|Default|SetCurrentHealth (- (Variables|Default|GetCurrentHealth) Damage))
      (if (<= (Variables|Default|GetCurrentHealth) 0.0)
        (CallFunction|EnemyDead)))))

(event Custom|EnemyDead
  ;[1 1 1] Damage System
  (Variables|Default|SetIsEnemyDead? true)
  (Variables|Default|SetIsReadyToFight false)
  (Variables|/Script/AIModule.PawnSensingComponent|SetbSeePawns (Variables|Default|GetPawnSensing) false)
  (Components|Movement|StopMovementImmediately (Variables|Character|GetCharacterMovement))
  (Actor|DestroyActor))

(event Custom|LookAt
  ;[1 1 1] Look At Player
  (Utilities|FlowControl|DoOnce false
    (:Completed
      (if (not (Variables|Default|GetIsEnemyDead?)) :!label _label
        (Transformation|SetActorRotation (Math|Rotator|MakeRotator 0.0 0.0 (.yaw (Math|Interpolation|RInterpTo (Transformation|GetActorRotation) (Math|Rotator|FindLookatRotation (Transformation|GetActorLocation) (Transformation|GetActorLocation (Game|GetPlayerCharacter 0))) (Utilities|Time|GetWorldDeltaSeconds) 3.0))))
        (Utilities|FlowControl|Delay 0.01)
        (goto _label)))))

(event Custom|StartTransform)

(event Custom|Floating
  (bind _smoke (Variables|Default|GetSmoke))
  (bind _relativelocation (Variables|/Script/Engine.SceneComponent|GetRelativeLocation _smoke))
  (bind _float (Timeline|FloatTimeline PlayFromStart)
    (:Update
      (Transformation|SetRelativeLocation _smoke (Math|Vector|MakeVector (.x _relativelocation) (.y _relativelocation) _float) false false))
    (:Finished
      (Utilities|FlowControl|Delay 0.01)
      (CallFunction|Floating))))

(event Custom|WBPEnemy
  ;[1 1 1] WBP
  (bind _aswbp_enemy_health (Utilities|Casting|CastToWBP_EnemyHealth (UserInterface|GetUserWidgetObject (Variables|Default|GetHealthWidget))))
  (Variables|/Game/Enemies/Blueprints/WBP_EnemyHealth.WBP_EnemyHealth_C|SetEnemy%20Ref _aswbp_enemy_health self)
  (Utilities|Time|SetTimerbyEvent (delegate Custom|CheckEnHealthWidget) 0.02 true))

(event Custom|CheckEnHealthWidget
  (bind _healthwidget (Variables|Default|GetHealthWidget))
  (bind _healthwidget_2 (Variables|Default|GetHealthWidget))
  ;[1 1 1] WBP
  (if (Variables|Default|GetIsReadyToFight)
    (if (Variables|Default|GetIsEnemyDead?)
      (Development|SetHiddeninGame _healthwidget_2 true false)
      (else
        (Development|SetHiddeninGame _healthwidget_2 false false)
        (bind _asbp_third_person_character (Utilities|Casting|CastToBP_ThirdPersonCharacter (Game|GetPlayerCharacter 0)))
        (Transformation|SetWorldRotation _healthwidget (Math|Rotator|MakeRotator 0.0 0.0 (.yaw (Math|Rotator|FindLookatRotation (Transformation|GetWorldLocation _healthwidget) (Transformation|GetWorldLocation (Variables|/Game/ThirdPerson/Blueprints/BP_ThirdPersonCharacter.BP_ThirdPersonCharacter_C|GetFollowCamera _asbp_third_person_character))))) false false)))
    (else
      (Development|SetHiddeninGame _healthwidget_2 true false))))

(event EventBeginPlay
  (CallFunction|Floating)
  (CallFunction|WBPEnemy))

(fn ConstructionScript)