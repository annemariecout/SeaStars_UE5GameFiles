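; Enemy projectile that homes in on the player character and deals point damage when it hits.
; On BeginPlay it targets the player's capsule through ProjectileMovement homing, and a looping timer switches homing off after a short delay.
; A sphere collision hit on the player applies damage, destroys the projectile and calls the character's death function if health equals zero.
; Hits on other actors are ignored by the graph.
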(event OnComponentHit(SphereCollision)
  (params (HitComponent :type Primitive%20Component%20Object%20Reference) (OtherActor :type Actor%20Object%20Reference) (OtherComp :type Primitive%20Component%20Object%20Reference) (NormalImpulse :type Vector :default "0, 0, 0") (Hit :type Hit%20Result%20Structure%20%28by%20ref%29))
  (bind _tp_char_ref (Variables|Default|GetTP%20Char%20Ref))
  ;[1 1 1] Hit
  (if (== OtherActor _tp_char_ref)
    (Game|Damage|ApplyPointDamage _tp_char_ref 1e+01 (.ImpactPoint (Collision|BreakHitResult Hit)) Hit 0 self)
    (Utilities|FlowControl|Sequence
      (:then_0
        (Actor|DestroyActor))
      (:then_1
        (if (== (Variables|/Game/ThirdPerson/Blueprints/BP_ThirdPersonCharacter.BP_ThirdPersonCharacter_C|GetHealthAmt (Variables|Default|GetTP%20Char%20Ref)) 0.0)
          (Default|TPCharDead (Variables|Default|GetTP%20Char%20Ref)))))))

(event Custom|HomeToPlayer
  (bind _projectilemovement (Variables|Default|GetProjectileMovement))
  ;[1 1 1] Home to Player
  (bind _asbp_third_person_character (Utilities|Casting|CastToBP_ThirdPersonCharacter (Game|Player|GetPlayerPawn 0)))
  (Variables|Default|SetTP%20Char%20Ref _asbp_third_person_character)
  (Variables|/Script/Engine.ProjectileMovementComponent|SetHomingTargetComponent _projectilemovement (Variables|/Script/Engine.Character|GetCapsuleComponent _asbp_third_person_character))
  (Variables|/Script/Engine.ProjectileMovementComponent|SetbIsHomingProjectile _projectilemovement true)
  (Variables|/Script/Engine.ProjectileMovementComponent|SetHomingAccelerationMagnitude _projectilemovement 2e+03))

(event Custom|DisableHoming
  ;[1 1 1] Disable Homing
  (Variables|/Script/Engine.ProjectileMovementComponent|SetbIsHomingProjectile (Variables|Default|GetProjectileMovement) false))

(event EventBeginPlay
  ;[1 1 1] Init
  (CallFunction|HometoPlayer)
  (Utilities|Time|SetTimerbyFunctionName 0 "DisableHoming" 1.8 true))

(fn ConstructionScript)